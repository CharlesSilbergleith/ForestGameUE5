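; BPC_DamageSystem is an Actor Component that tracks health, healing and death for its owner.
; TakeDamage passes a damage info struct's flags through the CanBeDamaged macro, which weighs death, invincibility, parry and block.
; Blocks fire OnBlocked; damage lowers health, then fires OnDeath or, if interruptible or forced, OnDamageResponce.
; The parry outcome is left unhandled in TakeDamage, and Heal clamps health to MaxHealth while alive.
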(fn `Heal`
  (params (amount :type "Float (double-precision)"))
  (returns (newhealth :type "Float (double-precision)"))
  (if (not (`self.IsDead`))
    (bind _output_get (set `self.Health` (`KismetMathLibrary.FClamp` (+ amount (`self.Health`)) 0.0 (`self.MaxHealth`))))
    (return _output_get)))

(fn `NewFunction_0`)

(fn `takeDamage`
  (params (DamageInfo :type "/Game/DamgeSystem/S_damageInfo Structure"))
  (returns (wasDamaged :type Boolean))
  (bind (_ammount _damagetype _damgaeresponce _blocking _dodge _parry _shoulddamgeinvinsable _canbeblocked _canbeparry _shouldforceinterupt) (break `/Game/DamgeSystem/S_damageInfo` DamageInfo))
  (`self.CanBeDamaged` _shoulddamgeinvinsable _canbeblocked _canbeparry
    (:`BlockDamage`
      (`self.OnBlocked` _canbeparry)
      (return false))
    (:`DoDamage`
      (if (not (`self.IsDead`))
        (bind _output_get (set `self.Health` (- (`self.Health`) _ammount)))
        (bind _output_get_2 (set `self.IsDead` (<= _output_get 0.0)))
        (if _output_get_2
          (`self.OnDeath`)
          (return true)
          (elif (or (`self.isInterupatble`) _shouldforceinterupt)
            (`self.OnDamageResponce` _damgaeresponce)
            (return true)))))))